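; BP_watch is a simple stopwatch Blueprint that shows elapsed time as a debug print.
; Tick accumulates DeltaSeconds into a Seconds variable and derives whole minutes by division and leftover seconds by modulo.
; It reprints the result every frame with Russian unit labels and a very short duration.
; The minutes calculation adds the current frame's DeltaSeconds again to the already updated total.
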(event EventBeginPlay)

(event Collision|EventActorBeginOverlap
  (params (OtherActor :type Actor%20Object%20Reference)))

(event EventTick
  (params (DeltaSeconds :type Float%20%28single-precision%29))
  (bind _output_get (Variables|Default|SetSeconds (+ DeltaSeconds (Variables|Default|GetSeconds))))
  (Development|PrintString (Utilities|String|Append (Utilities|String|ToString(Integer) (Math|Float|Truncate (/ (+ DeltaSeconds (Variables|Default|GetSeconds)) 6e+01))) "  мин " (Utilities|String|ToString(Integer) (Math|Float|Truncate (Math|Float|%(Float) _output_get 6e+01))) " сек") true true "(R=1.000000,G=0.000000,B=0.969102,A=1.000000)" 0.005))

(fn ConstructionScript)