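; BP_travel_cart is an actor Blueprint for a travel cart that spends tickets when something overlaps it, with no movement logic.
; Each unfiltered begin-overlap decrements a nonzero NumberOfTickets and prints the remaining count, followed by a separate label string.
; Using the last ticket and overlapping with none left share the same "No tickets left" message.
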(event EventBeginPlay)

(event EventTick
  (params (DeltaSeconds :type Float%20%28single-precision%29)))

(event Collision|EventActorBeginOverlap
  (params (OtherActor :type Actor%20Object%20Reference))
  (if (Math|Conversions|ToBoolean(Integer) (Variables|Default|GetNumber%20Of%20Tickets))
    (Variables|Default|SetNumberOfTickets (- (Variables|Default|GetNumber%20Of%20Tickets) 1))
    (if (> (Variables|Default|GetNumber%20Of%20Tickets) 0)
      (Development|PrintString (Utilities|String|ToString(Integer) (Variables|Default|GetNumber%20Of%20Tickets)))
      (Development|PrintString "Tickets Left:")
      (else
        (Development|PrintString "No tickets left" :!label _label)))
    (else
      (goto _label))))

(fn ConstructionScript)